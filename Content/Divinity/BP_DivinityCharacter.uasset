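; Player character Blueprint that equips a weapon and can spawn echo clones of itself.
; On BeginPlay it spawns BP_Weapon and attaches it to the right-hand socket.
; SpawnClones places an echo at a character-relative offset and yaw with a given montage, while SpawnWalkingClone scatters walking echoes randomly nearby.
; An unconnected walk-mode toggle would switch speed and loop a timer spawning walking clones in pairs.
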(event Custom|ClonesWalking
  ;[0.15 0.15 0.15 0.5] Walk Mode Input
  (CallFunction|SpawnWalkingClone)
  (Utilities|FlowControl|Delay 0.5)
  (CallFunction|SpawnWalkingClone))

(event EventBeginPlay
  (bind _returnvalue (Game|SpawnActorfromClass "/Game/Divinity/Blueprints/BP_Weapon.BP_Weapon_C" (Transformation|GetSocketTransform (Variables|Character|GetMesh) "Weapon_RSocket" "RTS_World") "Undefined" "MultiplyWithRoot" 0 0))
  (Transformation|AttachComponentToComponent _returnvalue (Variables|Character|GetMesh) "Weapon_RSocket" "SnapToTarget" "SnapToTarget" "SnapToTarget" true))

(event EventTick
  (params (DeltaSeconds :type Float%20%28single-precision%29)))

(fn ConstructionScript
  (|CallParentFunction))

(fn SpawnClones
  (params (ForwardOffset :type Float%20%28double-precision%29) (RightOffset :type Float%20%28double-precision%29) (RotationFromCharacter :type Float%20%28double-precision%29) (AnimMontage :type Anim%20Montage%20Object%20Reference))
  (bind _capsulecomponent (Variables|Default|GetCapsuleComponent))
  (LocalVariables|SetLocalForwardOffset ForwardOffset)
  (LocalVariables|SetLocalRightOffset RightOffset)
  (LocalVariables|SetLocalRoationFromCharacter RotationFromCharacter)
  (Utilities|IsValid AnimMontage
    (:Is%20Valid
      (LocalVariables|SetLocalAnimMontage AnimMontage)
      (Game|SpawnActorfromClass "/Game/Divinity/Blueprints/CombatAnimationBlueprints/BP_EchoSpawn.BP_EchoSpawn_C" (Math|Transform|MakeTransform (+ (+ (* (Math|Vector|GetForwardVector _capsulecomponent) (LocalVariables|GetLocalForwardOffset)) (* (Math|Vector|GetRightVector _capsulecomponent) (LocalVariables|GetLocalRightOffset))) (Transformation|GetActorLocation)) (Math|Rotator|MakeRotator 0.0 0.0 (+ (.yaw (Transformation|GetActorRotation)) (LocalVariables|GetLocalRoationFromCharacter))) "1.000000,1.000000,1.000000") "AdjustIfPossibleButAlwaysSpawn" "MultiplyWithRoot" 0 (LocalVariables|GetLocalAnimMontage) 0))))

(fn SpawnWalkingClone
  (bind _returnvalue (Math|Random|RandomFloatinRange -3e+02 3e+02))
  (bind _capsulecomponent (Variables|Default|GetCapsuleComponent))
  (Game|SpawnActorfromClass "/Game/Divinity/Blueprints/CombatAnimationBlueprints/BP_EchoSpawnWalking.BP_EchoSpawnWalking_C" (Math|Transform|MakeTransform (+ (+ (* (Math|Vector|GetForwardVector _capsulecomponent) _returnvalue) (* (Math|Vector|GetRightVector _capsulecomponent) _returnvalue)) (Transformation|GetActorLocation)) (Transformation|GetActorRotation) "1.000000,1.000000,1.000000") "AdjustIfPossibleButAlwaysSpawn" "MultiplyWithRoot" 0 "/Game/SwordAnimsetPro/Animations/Root-Motion/AnimationMontages/Walk_F_Anim_Montage.Walk_F_Anim_Montage" 0))

(fn Quit
  (Game|QuitGame 0 "Quit" false))