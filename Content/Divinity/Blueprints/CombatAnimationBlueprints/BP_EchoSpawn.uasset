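; BP_EchoSpawn is a short-lived echo clone that appears with a damage Niagara effect and plays a combat animation.
; BeginPlay snaps it to the ground with a downward trace offset by capsule height, and attaches a cloned weapon to the hand socket.
; Timelines drive dynamic fade materials on body and sword in, then back out after a delay, before the actor destroys itself.
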(event Custom|SnapToGround
  (bind _returnvalue (Transformation|GetActorLocation))
  (bind _returnvalue_2 (Transformation|GetActorLocation))
  (bind (_x _y) (Math|Vector|BreakVector _returnvalue_2))
  ;[0.15 0.15 0.15 0.5] Snap Clone to the Ground
  (Utilities|FlowControl|Delay 0.0)
  (bind _outhit (Collision|LineTraceByChannel _returnvalue_2 (Math|Vector|MakeVector _x _y (.z (+ _returnvalue_2 (* (Math|Vector|GetUpVector (Transformation|GetActorRotation)) -5e+02)))) "TraceTypeQuery1" false 0 "None"))
  (Transformation|SetActorLocation (Math|Vector|MakeVector (.x _returnvalue) (.y _returnvalue) (+ (.Z (Math|Vector|BreakVector (.ImpactPoint (Collision|BreakHitResult _outhit)))) (+ (Components|Capsule|GetScaledCapsuleHalfHeight (Variables|Collision|GetCapsuleComponent)) 1e+01))) false false))

(event EventBeginPlay
  (CallFunction|SnaptoGround)
  (Niagara|SpawnSystematLocation "/Game/Variant_Combat/VFX/NS_Damage.NS_Damage" (Transformation|GetActorLocation) (Transformation|GetActorRotation))
  (Components|Animation|PlayAnimation (Variables|Character|GetMesh) (Variables|Default|GetAnimationMontage) false)
  (bind _returnvalue (Game|SpawnActorfromClass "/Game/Divinity/Blueprints/BP_WeaponClones.BP_WeaponClones_C" (Transformation|GetSocketTransform (Variables|Character|GetMesh) "Weapon_RSocket" "RTS_World") "Undefined" "MultiplyWithRoot" 0 0))
  (Transformation|AttachComponentToComponent _returnvalue (Variables|Character|GetMesh) "Weapon_RSocket" "SnapToTarget" "SnapToTarget" "SnapToTarget" true)
  (bind _returnvalue_2 (Rendering|Material|CreateDynamicMaterialInstance (Variables|/Game/Divinity/Blueprints/BP_WeaponClones.BP_WeaponClones_C|GetSkeletalMesh _returnvalue) 0 "/Game/SwordAnimsetPro/Demo/Character/Materials/M_Weapon_SwrodFade.M_Weapon_SwrodFade" "None" :!class /Script/Engine.PrimitiveComponent))
  (bind _returnvalue_3 (Rendering|Material|CreateDynamicMaterialInstance (Variables|Character|GetMesh) 0 "/Game/Divinity/NiagaraEffects/Materials/MI_Body_Fade_Inst.MI_Body_Fade_Inst" "None" :!class /Script/Engine.PrimitiveComponent))
  (bind _fadetimecurve (Timeline|FadeInTimeline PlayFromStart)
    (:Update
      (Rendering|Material|SetScalarParameterValue _returnvalue_3 "Fade" _fadetimecurve :!class /Script/Engine.MaterialInstanceDynamic)
      (Rendering|Material|SetScalarParameterValue _returnvalue_2 "SwordFadeOpacity" _fadetimecurve :!class /Script/Engine.MaterialInstanceDynamic)
      (Utilities|FlowControl|Delay 0.8)
      (bind _fadetimecurve_2 (Timeline|FadeOutTimeline ReverseFromEnd)
        (:Update
          (Rendering|Material|SetScalarParameterValue _returnvalue_3 "Fade" _fadetimecurve_2 :!class /Script/Engine.MaterialInstanceDynamic)
          (Rendering|Material|SetScalarParameterValue _returnvalue_2 "SwordFadeOpacity" _fadetimecurve_2 :!class /Script/Engine.MaterialInstanceDynamic))
        (:Finished
          (Utilities|FlowControl|Delay 2.0)
          (Actor|DestroyActor))))))

(fn ConstructionScript)