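; BP_EchoSpawnWalking is a short-lived echo clone that glides forward, carrying a cloned weapon, while fading in and out.
; On BeginPlay it attaches a BP_WeaponClones to its right-hand weapon socket and creates dynamic fade materials for body and sword.
; Chained timelines drive both fades, then the clone destroys itself after a short delay.
; Tick moves it at constant speed, using a downward line trace to keep it grounded.
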(event Custom|SnapToGround
  (bind _returnvalue (Transformation|GetActorLocation))
  (bind _returnvalue_2 (Transformation|GetActorLocation))
  (bind (_x _y) (Math|Vector|BreakVector _returnvalue_2))
  ;[0.15 0.15 0.15 0.5] Snap Clone to the Ground
  (Utilities|FlowControl|Delay 0.0)
  (bind _outhit (Collision|LineTraceByChannel _returnvalue_2 (Math|Vector|MakeVector _x _y (.z (+ _returnvalue_2 (* (Math|Vector|GetUpVector (Transformation|GetActorRotation)) -5e+02)))) "TraceTypeQuery1" false 0 "None"))
  (Transformation|SetActorLocation (Math|Vector|MakeVector (.x _returnvalue) (.y _returnvalue) (+ (.Z (Math|Vector|BreakVector (.ImpactPoint (Collision|BreakHitResult _outhit)))) (+ (Components|Capsule|GetScaledCapsuleHalfHeight (Variables|Collision|GetCapsuleComponent)) 1e+01))) false false))

(event EventBeginPlay
  (CallFunction|SnaptoGround)
  (bind _returnvalue (Game|SpawnActorfromClass "/Game/Divinity/Blueprints/BP_WeaponClones.BP_WeaponClones_C" (Transformation|GetSocketTransform (Variables|Character|GetMesh) "Weapon_RSocket" "RTS_World") "Undefined" "MultiplyWithRoot" 0 0))
  (Transformation|AttachComponentToComponent _returnvalue (Variables|Character|GetMesh) "Weapon_RSocket" "SnapToTarget" "SnapToTarget" "SnapToTarget" true)
  (bind _returnvalue_2 (Rendering|Material|CreateDynamicMaterialInstance (Variables|/Game/Divinity/Blueprints/BP_WeaponClones.BP_WeaponClones_C|GetSkeletalMesh _returnvalue) 0 "/Game/SwordAnimsetPro/Demo/Character/Materials/M_Weapon_SwrodFade.M_Weapon_SwrodFade" "None" :!class /Script/Engine.PrimitiveComponent))
  (Variables|Default|SetSwordMaterial _returnvalue_2)
  (bind _returnvalue_3 (Rendering|Material|CreateDynamicMaterialInstance (Variables|Character|GetMesh) 0 "/Game/Divinity/NiagaraEffects/Materials/MI_Body_Fade_Inst.MI_Body_Fade_Inst" "None" :!class /Script/Engine.PrimitiveComponent))
  (Variables|Default|SetBodyMaterial _returnvalue_3)
  (bind _fadetimecurve (Timeline|FadeInTimeline PlayFromStart)
    (:Update
      (Rendering|Material|SetScalarParameterValue (Variables|Default|GetBodyMaterial) "Fade" _fadetimecurve :!class /Script/Engine.MaterialInstanceDynamic)
      (Rendering|Material|SetScalarParameterValue (Variables|Default|GetSwordMaterial) "SwordFadeOpacity" _fadetimecurve :!class /Script/Engine.MaterialInstanceDynamic))
    (:Finished
      (bind _fadetimecurve_2 (Timeline|FadeOutTimeline ReverseFromEnd)
        (:Update
          (Rendering|Material|SetScalarParameterValue (Variables|Default|GetBodyMaterial) "Fade" _fadetimecurve_2 :!class /Script/Engine.MaterialInstanceDynamic)
          (Rendering|Material|SetScalarParameterValue (Variables|Default|GetSwordMaterial) "SwordFadeOpacity" _fadetimecurve_2 :!class /Script/Engine.MaterialInstanceDynamic))
        (:Finished
          (Utilities|FlowControl|Delay 1.0)
          (Actor|DestroyActor))))))

(event EventTick
  (params (DeltaSeconds :type Float%20%28single-precision%29))
  (Transformation|AddActorWorldOffset (* (* (Math|Vector|GetForwardVector (Variables|Collision|GetCapsuleComponent)) 2e+02) DeltaSeconds))
  (CallFunction|SnaptoGround))

(fn ConstructionScript)