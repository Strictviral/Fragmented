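; Gameplay ability that listens on a player clone for a teleport-attack event and performs a surprise strike on the event's target.
; It teleports the clone to a random nav-projected point around the target, facing it, reverses the dissolve and plays a random attack montage.
; On authority, hit-scan events toggle the clone weapon's trace, passing a SetByCaller damage spec.
; MontageStarted is an empty hook for child abilities.
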(event Custom|HandleHitScanStart
  ;[0.15 0.15 0.15 0.5] HitScanEvents
  (bind _cloneweapon (Variables|Default|GetCloneWeapon)
    (:then
      (bind _returnvalue (Ability|GameplayEffect|AssignTagSetbyCallerMagnitude (Ability|MakeOutgoingGameplayEffectSpec (Variables|GameplayEffect|GetGameplay%20Effect%20Class)) "(TagName=\"Data.Damage\")" (Variables|GameplayEffect|GetDamageMagnitude)))
      (Default|HitScanStart _cloneweapon _returnvalue))
    (:else)))

(event Custom|HandleHitScanEnd
  ;[0.15 0.15 0.15 0.5] HitScanEvents
  (bind _cloneweapon (Variables|Default|GetCloneWeapon)
    (:then
      (Default|HitScanEnd _cloneweapon))
    (:else)))

(event Custom|MontageStarted
  ;[0.15 0.15 0.15 0.5] Override In Child
)

(event Custom|TeleportToEnemy
  (params (Actor :type Actor%20Object%20Reference))
  (bind _returnvalue (Transformation|GetActorLocation Actor))
  (bind _returnvalue_2 (Math|Random|RandomUnitVector))
  (bind _returnvalue_3 (Math|Vector|MakeVector (.x _returnvalue_2) (.y _returnvalue_2) 0.0))
  (bind _returnvalue_4 (Math|Vector|Normalize _returnvalue_3))
  (bind _returnvalue_5 (* _returnvalue_4 5e+02))
  (bind _returnvalue_6 (+ _returnvalue_5 _returnvalue))
  (bind _returnvalue_7 (Math|Rotator|FindLookatRotation _returnvalue_6 _returnvalue))
  (bind _projectedlocation (AI|Navigation|ProjectPointtoNavigation _returnvalue_6 0 0 "100.000000,100.000000,200.000000"))
  (Transformation|Teleport (Ability|GetAvatarActorfromActorInfo) (Math|Vector|MakeVector (.x _projectedlocation) (.y _projectedlocation) (.z _projectedlocation)) (Math|Rotator|MakeRotator (.roll _returnvalue_7) 0.0 (.yaw _returnvalue_7))))

(event Ability|EventActivateAbility
  (bind _asbp_fragmented_player_clone (Utilities|Casting|CastToBP_FragmentedPlayerClone (Ability|GetAvatarActorfromActorInfo)))
  (bind _output_get (Variables|Default|SetAs%20BP%20Fragmented%20Player%20Clone _asbp_fragmented_player_clone))
  (Utilities|IsValid (Variables|/Game/Fragmented/Characters/BP_FragmentedPlayerClone.BP_FragmentedPlayerClone_C|GetWeapon _output_get)
    (:Is%20Valid
      (Variables|Default|SetCloneWeapon (Variables|/Game/Fragmented/Characters/BP_FragmentedPlayerClone.BP_FragmentedPlayerClone_C|GetWeapon _output_get))
      (bind _payload (Ability|Tasks|WaitGameplayEvent "(TagName=\"GameplayAbility.Clone.TeleportAttack\")" 0)
        (:then
          (Ability|Tasks|WaitGameplayEvent "(TagName=\"GameplayAbility.Clone.BasicAttack\")" 0))
        (:EventReceived
          (CallFunction|TeleporttoEnemy (.target _payload))
          (Default|ReverseDissolve (Variables|Default|GetAs%20BP%20Fragmented%20Player%20Clone))
          (|PlayMontageandWaitProxy "None" (Utilities|Array|Get(acopy) (Variables|Animation|GetAttackMontage) (Math|Random|RandomIntegerinRange 0 (CallFunction|ReturnLengthOfAnimationArray))) 1.0 "None" true 1.0 0.0 false
            (:then
              (CallFunction|MontageStarted)
              (Ability|HasAuthority
                (:True
                  (Ability|Tasks|WaitGameplayEvent "(TagName=\"Event.HitScan.Start\")" 0
                    (:then
                      (Ability|Tasks|WaitGameplayEvent "(TagName=\"Event.HitScan.End\")" 0
                        (:EventReceived
                          (CallFunction|HandleHitScanEnd))))
                    (:EventReceived
                      (CallFunction|HandleHitScanStart))))))))))
    (:Is%20Not%20Valid
      (Ability|EndAbility))))

(fn ReturnLengthOfAnimationArray
  (return (- (Utilities|Array|Length (Variables|Animation|GetAttackMontage)) 1)))