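; Gameplay ability that removes a player clone from the world with an animated exit and dissolve.
; It plays an attack combo montage on the avatar clone and listens for the fade-out gameplay event, which triggers the dissolve and the clone weapon's death handling.
; Montage blend-out or completion runs the clone actor's death handling; the graph never calls EndAbility itself.
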(event Ability|EventActivateAbility
  (bind _asbp_fragmented_player_clone (Utilities|Casting|CastToBP_FragmentedPlayerClone (Ability|GetAvatarActorfromActorInfo)))
  (Variables|Default|SetAs%20BP%20Fragmented%20Player%20Clone _asbp_fragmented_player_clone)
  (|PlayMontageandWaitProxy "None" "/Game/SwordAnimsetPro/Animations/Root-Motion/AnimationMontages/Combo2/Attack_Combo_02_04_Anim_Montage.Attack_Combo_02_04_Anim_Montage" 1.0 "None" true 1.0 0.0 false
    (:then
      (Ability|Tasks|WaitGameplayEvent "(TagName=\"GameplayAbility.Effect.Fade.OUT\")" 0
        (:EventReceived
          (Default|Dissolve (Variables|Default|GetAs%20BP%20Fragmented%20Player%20Clone))
          (Default|HandleDeathCustomBlueprintCloneWeapon (Variables|Default|GetAs%20BP%20Fragmented%20Player%20Clone)))))
    (:OnCompleted
      (Default|HandleDeathCustomBlueprintCloneActor (Variables|Default|GetAs%20BP%20Fragmented%20Player%20Clone) :!label _label))
    (:OnBlendOut
      (goto _label))))

(event Ability|EventOnEndAbility
  (params (bWasCancelled :type Boolean)))