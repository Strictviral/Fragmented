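; Boss gameplay ability that fires a damaging projectile, timed to a montage gameplay event and ending with the montage.
; With a valid attack-target message it aims at the player location captured on activation; otherwise, given a player controller, it uses an instant line-trace endpoint.
; The projectile spawns authority-only from the boss's spawn point or actor location, carrying a SetByCaller damage spec and boss spawn/impact GameplayCues.
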(event Custom|ShootProjectile
  (params (TargetLocation :type Vector))
  (bind _returnvalue (Ability|GameplayEffect|AssignTagSetbyCallerMagnitude (Ability|MakeOutgoingGameplayEffectSpec (Variables|Default|GetGameplay%20Effect%20Class)) "(TagName=\"Data.Damage\")" (Variables|Default|GetDamage%20Magnitude)))
  (bind _location (CallFunction|GetSpawnLocation))
  (|SpawnActor 0 _location "0, 0, 0" (Variables|Default|GetProjectile%20Class) true (Variables|Default|GetSpeed) TargetLocation _returnvalue "(TagName=\"GameplayCue.ProjectileSpawn.Boss\")" "(TagName=\"GameplayCue.ProjectileImpact.Boss\")" (.AsPawn (Utilities|Casting|CastToPawn (Ability|GetAvatarActorfromActorInfo)))))

(event Ability|EventActivateAbility
  (|CallParentFunction)
  (Utilities|Casting|CastToBP_EnemyBase (Ability|GetAvatarActorfromActorInfo))
  (Variables|Default|SetPlayerLocation (Transformation|GetActorLocation (Game|Player|GetPlayerPawn 0)))
  (Ability|CommitAbilityCooldown false)
  (|PlayMontageandWaitProxy "None" (Variables|Default|GetMontage%20to%20Play) 1.0 "None" true 1.0 0.0 false
    (:then
      (Ability|Tasks|WaitGameplayEvent "(TagName=\"Event.Montage.Trigger\")" 0
        (:EventReceived
          (bind _attacktarget (Class|BPITargeting|GetAttackTarget(Message) (Ability|GetAvatarActorfromActorInfo)))
          (Utilities|IsValid _attacktarget
            (:Is%20Valid
              (CallFunction|ShootProjectile (Variables|Default|GetPlayerLocation)))
            (:Is%20Not%20Valid
              (if (Class|FragmentedGameplayAbility|HasPC)
                (bind _data (|WaitTargetData :ConfirmationType "Instant" :Class "/Script/GameplayAbilities.GameplayAbilityTargetActor_SingleLineTrace" :TraceProfile "(Name=\"NoCollision\")" :StartLocation (Class|GameplayAbility|MakeTargetLocationInfofromOwnerActor) :ReticleClass 0)
                  (:ValidData
                    (CallFunction|ShootProjectile (Class|AbilitySystemBlueprintLibrary|GetTargetDataEndPoint _data))))))))))
    (:OnCompleted
      (Ability|EndAbility :!label _label))
    (:OnInterrupted
      (goto _label))))

(event Ability|EventOnEndAbility
  (params (bWasCancelled :type Boolean))
  (|CallParentFunction bWasCancelled) ; This node is disabled and will not be called.\nDrag off pins to build functionality.
)

(fn GetSpawnLocation
  (bind _returnvalue (Ability|GetAvatarActorfromActorInfo))
  (bind _asbp_boss_enemy (Utilities|Casting|CastToBP_BossEnemy _returnvalue))
  (Utilities|IsValid _asbp_boss_enemy
    (:Is%20Valid
      (return (Default|GetSpawnLocation _asbp_boss_enemy)))
    (:Is%20Not%20Valid
      (return (Transformation|GetActorLocation (Ability|GetAvatarActorfromActorInfo))))))