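; Gameplay ability that runs the death sequence for enemies derived from BP_EnemyBase.
; If the enemy has a death reaction montage, it applies GE_Death to itself and plays that montage; otherwise the ability ends immediately.
; An Event.Montage.Death gameplay event during playback triggers the enemy's Dissolve.
; Montage completion calls DeathAnimationFinished and ends the ability.
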(event Ability|EventActivateAbility
  (bind _asbp_enemy_base (Utilities|Casting|CastToBP_EnemyBase (Ability|GetAvatarActorfromActorInfo)))
  (Variables|Default|SetAs%20BP%20Enemy%20Base _asbp_enemy_base)
  (Utilities|IsValid (Variables|/Script/Fragmented.FragmentedCharacterBase|GetDeathReactionMontage _asbp_enemy_base)
    (:Is%20Valid
      (Ability|ApplyGameplayEffectToOwner "/Game/Fragmented/Effects/GE_Death.GE_Death_C")
      (|PlayMontageandWaitProxy "None" (Variables|/Script/Fragmented.FragmentedCharacterBase|GetDeathReactionMontage _asbp_enemy_base) 1.0 "None" true 1.0 0.0 false
        (:then
          (Ability|Tasks|WaitGameplayEvent "(TagName=\"Event.Montage.Death\")" 0
            (:EventReceived
              (Default|Dissolve (Variables|Default|GetAs%20BP%20Enemy%20Base)))))
        (:OnCompleted
          (Class|FragmentedEnemyCharacterBase|DeathAnimationFinished (Variables|Default|GetAs%20BP%20Enemy%20Base))
          (Ability|EndAbility))))
    (:Is%20Not%20Valid
      (Ability|EndAbility))))

(event Ability|EventOnEndAbility
  (params (bWasCancelled :type Boolean)))