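; Base melee attack Gameplay Ability for Fragmented enemies, playing an attack montage and driving the weapon's hit scan.
; On the authority, Event.HitScan.Start and End gameplay events open and close the scan, passing a SetByCaller damage effect spec to the weapon.
; The ability ends with the montage and stops any scan on end.
; MontageStarted is an empty child hook; an overridable SpawnClone event spawns a player clone but is not called here.
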(event Custom|HandleHitScanStart
  ;[0.15 0.15 0.15 0.5] HitScanEvents
  (bind _enemyweapon (Variables|Default|GetEnemyWeapon)
    (:then
      (bind _returnvalue (Ability|GameplayEffect|AssignTagSetbyCallerMagnitude (Ability|MakeOutgoingGameplayEffectSpec (Variables|GameplayEffect|GetGameplay%20Effect%20Class)) "(TagName=\"Data.Damage\")" (Variables|GameplayEffect|GetDamageMagnitude)))
      (Default|HitScanStart _enemyweapon _returnvalue))
    (:else)))

(event Custom|HandleHitScanEnd
  ;[0.15 0.15 0.15 0.5] HitScanEvents
  (bind _enemyweapon (Variables|Default|GetEnemyWeapon)
    (:then
      (Default|HitScanEnd _enemyweapon))
    (:else)))

(event Custom|MontageStarted
  ;[0.15 0.15 0.15 0.5] Override In Child
)

(event Custom|SpawnClone
  ;[0.15 0.15 0.15 0.5] Override in Child
  (bind _returnvalue (Game|SpawnActorfromClass "/Game/Fragmented/Characters/BP_FragmentedPlayerClone.BP_FragmentedPlayerClone_C" (Transformation|GetActorTransform (Variables|Default|GetAs%20BP%20Fragmented%20Player)) "Undefined" "MultiplyWithRoot" 0 0))
  (Variables|Default|SetPlayerClone _returnvalue))

(event Ability|EventActivateAbility
  (bind _asbp_fragmented_enemy_base (Utilities|Casting|CastToBP_FragmentedEnemyBase (Ability|GetAvatarActorfromActorInfo)))
  (bind _output_get (Variables|Default|SetAs%20BP%20Fragmented%20Enemy%20Base _asbp_fragmented_enemy_base))
  (Utilities|IsValid (Variables|/Game/Fragmented/Characters/BP_FragmentedEnemyBase.BP_FragmentedEnemyBase_C|GetWeapon _output_get)
    (:Is%20Valid
      (Variables|Default|SetEnemyWeapon (Variables|/Game/Fragmented/Characters/BP_FragmentedEnemyBase.BP_FragmentedEnemyBase_C|GetWeapon _output_get))
      (bind _attackmontage (Variables|Animation|GetAttackMontage)
        (:then
          (|PlayMontageandWaitProxy "None" _attackmontage 1.0 "None" true 1.0 0.0 false
            (:then
              (CallFunction|MontageStarted)
              (Ability|HasAuthority
                (:True
                  (Ability|Tasks|WaitGameplayEvent "(TagName=\"Event.HitScan.Start\")" 0
                    (:then
                      (Ability|Tasks|WaitGameplayEvent "(TagName=\"Event.HitScan.End\")" 0
                        (:EventReceived
                          (CallFunction|HandleHitScanEnd))))
                    (:EventReceived
                      (CallFunction|HandleHitScanStart))))))
            (:OnCompleted
              (Ability|EndAbility :!label _label))
            (:OnInterrupted
              (goto _label))
            (:OnCancelled
              (goto _label))))
        (:else
          (Ability|EndAbility :!label _label_2))))
    (:Is%20Not%20Valid
      (goto _label_2))))

(event Ability|EventOnEndAbility
  (params (bWasCancelled :type Boolean))
  (bind _enemyweapon (Variables|Default|GetEnemyWeapon)
    (:then
      (Default|HitScanEnd _enemyweapon))
    (:else)))