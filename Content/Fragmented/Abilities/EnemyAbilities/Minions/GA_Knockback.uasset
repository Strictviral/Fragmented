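; Gameplay ability for enemy minions that shoves the avatar away from an area-of-effect source.
; On activation it waits for a GameplayAbility.Knockback event and takes the payload's Instigator location as the blast origin.
; The normalized origin-to-avatar direction feeds a short, strong root motion constant force, using only its X and Y components.
; The ability never calls EndAbility, and the separate Knockback function is an unused stub that only computes the direction.
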(event Custom|ApplyForceKnockback
  (params (EnemyLocation :type Vector) (AOELocation :type Vector))
  (bind _normalizedirection (CallFunction|CalculateandReturnKnockBackDirection EnemyLocation AOELocation))
  (Ability|Tasks|ApplyRootMotionConstantForce "None" (Math|Vector|MakeVector (.x _normalizedirection) (.y _normalizedirection) 0.0) 5e+03 0.3 false 0 "SetVelocity"))

(event Ability|EventActivateAbility
  (|CallParentFunction)
  (bind _payload (Ability|Tasks|WaitGameplayEvent "(TagName=\"GameplayAbility.Knockback\")" 0)
    (:EventReceived
      (CallFunction|ApplyForceKnockback (Transformation|GetActorLocation (Ability|GetAvatarActorfromActorInfo)) (Transformation|GetActorLocation (.instigator _payload))))))

(event Ability|EventOnEndAbility
  (params (bWasCancelled :type Boolean))
  (|CallParentFunction bWasCancelled) ; This node is disabled and will not be called.\nDrag off pins to build functionality.
)

(fn CalculateandReturnKnockBackDirection
  (params (EnemyLocation :type Vector) (AOELocation :type Vector))
  (return (Math|Vector|Normalize (- EnemyLocation AOELocation))))

(fn Knockback
  (params (EnemyLocation :type Vector) (AOELocation :type Vector))
  (CallFunction|CalculateandReturnKnockBackDirection EnemyLocation AOELocation))