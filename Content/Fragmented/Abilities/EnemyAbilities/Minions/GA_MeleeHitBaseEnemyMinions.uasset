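; Base melee attack gameplay ability for minion enemies that plays the BP_MeleeEnemy's basic attack montage.
; On authority it waits for left, right and end HitScan gameplay events, starting the enemy's matching hit scan with a SetByCaller damage effect spec or stopping it.
; The montage finishing or being interrupted ends the ability, which also stops the hit scan.
; MontageStarted is an empty hook for child abilities to override.
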(event Custom|HandleHitScanStartL
  ;[0.15 0.15 0.15 0.5] HitScanEvents
  (bind _as_bp_melee_enemy (Variables|Default|GetAs%20BP%20Melee%20Enemy)
    (:then
      (bind _returnvalue (Ability|GameplayEffect|AssignTagSetbyCallerMagnitude (Ability|MakeOutgoingGameplayEffectSpec (Variables|GameplayEffect|GetGameplay%20Effect%20Class)) "(TagName=\"Data.Damage\")" (Variables|GameplayEffect|GetDamageMagnitude)))
      (Default|HitScanStartL _as_bp_melee_enemy _returnvalue))
    (:else)))

(event Custom|HandleHitScanEnd
  ;[0.15 0.15 0.15 0.5] HitScanEvents
  (bind _as_bp_melee_enemy (Variables|Default|GetAs%20BP%20Melee%20Enemy)
    (:then
      (Default|HitScanEnd _as_bp_melee_enemy))
    (:else)))

(event Custom|MontageStarted
  ;[0.15 0.15 0.15 0.5] Override In Child
)

(event Custom|HandleHitScanStartR
  ;[0.15 0.15 0.15 0.5] HitScanEvents
  (bind _as_bp_melee_enemy (Variables|Default|GetAs%20BP%20Melee%20Enemy)
    (:then
      (bind _returnvalue (Ability|GameplayEffect|AssignTagSetbyCallerMagnitude (Ability|MakeOutgoingGameplayEffectSpec (Variables|GameplayEffect|GetGameplay%20Effect%20Class)) "(TagName=\"Data.Damage\")" (Variables|GameplayEffect|GetDamageMagnitude)))
      (Default|HitScanStartR _as_bp_melee_enemy _returnvalue))
    (:else)))

(event Ability|EventActivateAbility
  (bind _asbp_melee_enemy (Utilities|Casting|CastToBP_MeleeEnemy (Ability|GetAvatarActorfromActorInfo)))
  (bind _output_get (Variables|Default|SetAs%20BP%20Melee%20Enemy _asbp_melee_enemy))
  (Utilities|IsValid (Variables|/Game/Fragmented/Characters/Enemies/BP_EnemyBase.BP_EnemyBase_C|GetBasicAttackAnimation _output_get)
    (:Is%20Valid
      (|PlayMontageandWaitProxy "None" (Variables|/Game/Fragmented/Characters/Enemies/BP_EnemyBase.BP_EnemyBase_C|GetBasicAttackAnimation _output_get) 1.0 "None" true 1.0 0.0 false
        (:then
          (CallFunction|MontageStarted)
          (Ability|HasAuthority
            (:True
              (Ability|Tasks|WaitGameplayEvent "(TagName=\"Event.HitScan.Start.L\")" 0
                (:then
                  (Ability|Tasks|WaitGameplayEvent "(TagName=\"Event.HitScan.Start.R\")" 0
                    (:then
                      (Ability|Tasks|WaitGameplayEvent "(TagName=\"Event.HitScan.End\")" 0
                        (:EventReceived
                          (CallFunction|HandleHitScanEnd))))
                    (:EventReceived
                      (Development|PrintString "start htiscan")
                      (CallFunction|HandleHitScanStartR))))
                (:EventReceived
                  (CallFunction|HandleHitScanStartL))))))
        (:OnCompleted
          (Ability|EndAbility :!label _label))
        (:OnInterrupted
          (goto _label))
        (:OnCancelled
          (goto _label))))
    (:Is%20Not%20Valid
      (Ability|EndAbility))))

(event Ability|EventOnEndAbility
  (params (bWasCancelled :type Boolean))
  (|CallParentFunction false)
  (bind _as_bp_melee_enemy (Variables|Default|GetAs%20BP%20Melee%20Enemy)
    (:then
      (Default|HitScanEnd _as_bp_melee_enemy))
    (:else)))