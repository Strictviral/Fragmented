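; Base Gameplay Ability for ranged minion attacks that fires a projectile on a montage trigger event.
; It aims at the avatar's attack target, or falls back to instant line-trace target data when a player controller exists.
; The authority-spawned projectile carries a SetByCaller damage effect spec and starts at the ranged enemy's spawn point or the avatar's location.
; The ability ends when the montage completes, blends out or is interrupted.
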(event Custom|ShootProjectile
  (params (TargetLocation :type Vector))
  (bind _returnvalue (Ability|GameplayEffect|AssignTagSetbyCallerMagnitude (Ability|MakeOutgoingGameplayEffectSpec (Variables|Default|GetGameplay%20Effect%20Class)) "(TagName=\"Data.Damage\")" (Variables|Default|GetDamage%20Magnitude)))
  (bind _location (CallFunction|GetSpawnLocation))
  (|SpawnActor :SpawnLocation _location :Class (Variables|Default|GetProjectile%20Class) :bSpawnOnlyOnAuthority true :Speed (Variables|Default|GetSpeed) :TargetLocation TargetLocation :Effect%20Spec%20Handle _returnvalue :Instigator (.AsPawn (Utilities|Casting|CastToPawn (Ability|GetAvatarActorfromActorInfo)))))

(event Ability|EventActivateAbility
  (|PlayMontageandWaitProxy "None" (Variables|Default|GetBase%20Montage) 1.0 "None" true 1.0 0.0 false
    (:then
      (Ability|Tasks|WaitGameplayEvent "(TagName=\"Event.Montage.Trigger\")" 0
        (:EventReceived
          (bind _attacktarget (Class|BPITargeting|GetAttackTarget(Message) (Ability|GetAvatarActorfromActorInfo)))
          (Utilities|IsValid _attacktarget
            (:Is%20Valid
              (CallFunction|ShootProjectile (Transformation|GetActorLocation _attacktarget)))
            (:Is%20Not%20Valid
              (if (Class|FragmentedGameplayAbility|HasPC)
                (bind _data (|WaitTargetData :ConfirmationType "Instant" :Class "/Script/GameplayAbilities.GameplayAbilityTargetActor_SingleLineTrace" :TraceProfile "(Name=\"NoCollision\")" :StartLocation (Class|GameplayAbility|MakeTargetLocationInfofromOwnerActor) :ReticleClass 0)
                  (:ValidData
                    (CallFunction|ShootProjectile (Class|AbilitySystemBlueprintLibrary|GetTargetDataEndPoint _data))))))))))
    (:OnCompleted
      (Ability|EndAbility :!label _label))
    (:OnBlendOut
      (goto _label))
    (:OnInterrupted
      (goto _label))))

(fn GetSpawnLocation
  (bind _returnvalue (Ability|GetAvatarActorfromActorInfo))
  (bind _asbp_ranged_enemy (Utilities|Casting|CastToBP_RangedEnemy _returnvalue))
  (Utilities|IsValid _asbp_ranged_enemy
    (:Is%20Valid
      (return (Default|GetSpawnPointLocation _asbp_ranged_enemy)))
    (:Is%20Not%20Valid
      (return (Transformation|GetActorLocation (Ability|GetAvatarActorfromActorInfo))))))