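; GA_EnemyGreenSpecialHeal is an enemy minion gameplay ability that drops a healing area to support its allies.
; On activation it gets the enemy AI controller, commits cooldown and plays a montage, ending when the montage finishes or is cut short.
; A montage trigger gameplay event spawns BP_EffectArea_Heal with an instant heal effect at the lowest-health ally found by the controller, falling back to the caster's location.
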(event Custom|SpawnHealingField
  (bind _lowesthealthally (Default|FindLowestHealthAlly (Variables|Default|GetAs%20AIC%20Enemy%20Base)))
  (Utilities|IsValid _lowesthealthally
    (:Is%20Valid
      (Variables|Default|SetHealingFieldSpawnLocation (Transformation|GetActorLocation _lowesthealthally)))
    (:Is%20Not%20Valid
      (Variables|Default|SetHealingFieldSpawnLocation (Transformation|GetActorLocation (Ability|GetAvatarActorfromActorInfo)))))
  (|SpawnActor :SpawnLocation (Variables|Default|GetHealingFieldSpawnLocation) :Class "/Game/Fragmented/EffectActors/BP_EffectArea_Heal.BP_EffectArea_Heal_C" :Gameplay%20Effect%20Class "/Game/Fragmented/Effects/GE_HealInstant.GE_HealInstant_C" :Instigator (.AsPawn (Utilities|Casting|CastToPawn (Ability|GetAvatarActorfromActorInfo)))))

(event Ability|EventActivateAbility
  (|CallParentFunction)
  (bind _asaic_enemy_base (Utilities|Casting|CastToAIC_Enemy_Base (AI|GetAIController (Ability|GetAvatarActorfromActorInfo))))
  (Utilities|IsValid _asaic_enemy_base
    (:Is%20Valid
      (Variables|Default|SetAs%20AIC%20Enemy%20Base _asaic_enemy_base)
      (Ability|CommitAbilityCooldown false)
      (|PlayMontageandWaitProxy "None" (Variables|Default|GetMontage%20to%20Play) 1.0 "None" true 1.0 0.0 false
        (:then
          (Ability|Tasks|WaitGameplayEvent "(TagName=\"Event.Montage.Trigger\")" 0
            (:EventReceived
              (CallFunction|SpawnHealingField))))
        (:OnCompleted
          (Ability|EndAbility :!label _label))
        (:OnInterrupted
          (goto _label))
        (:OnCancelled
          (goto _label))))
    (:Is%20Not%20Valid
      (Ability|EndAbility))))

(event Ability|EventOnEndAbility
  (params (bWasCancelled :type Boolean))
  (|CallParentFunction bWasCancelled))