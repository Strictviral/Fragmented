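; GAS teleport-strike ability that leaves a player clone at the origin and deals radial damage at the destination.
; An avatar-supplied attack target is ground-traced; otherwise, players aim with a decal target actor during a looping montage.
; After commit, it spawns the clone and indicator cue, then a montage event triggers the teleport, explosion cue and authority-only sphere-trace damage via SetByCaller.
; Targeting disables movement; the restore node is unwired.
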(event Custom|LoopTargetingAnimation
  ;[0.15 0.15 0.15 0.5] Phase 1
  (|PlayMontageandWaitProxy "None" "/Game/SwordAnimsetPro/Animations/In-Place/Buff_In_Anim_Montage.Buff_In_Anim_Montage" 0.5 "None" true 1.0 0.0 false
    (:OnCompleted
      _)
    (:OnBlendedIn
      _)
    (:OnBlendOut
      _))
  (|PlayMontageandWaitProxy "None" "/Game/SwordAnimsetPro/Animations/In-Place/Buff_Loop_Anim_Montage.Buff_Loop_Anim_Montage" 1.0 "None" true 1.0 0.0 false :!label _label
    (:OnBlendOut
      (if (Variables|Default|GetbIsWaitingTargetData)
        (goto _label)))
    (:OnInterrupted
      (if (Variables|Default|GetbIsWaitingTargetData)
        (Ability|EndAbility)))))

(event Custom|ConfirmStrike
  ;[0.15 0.15 0.15 0.5] Phase 2
  (bind _returnvalue (Ability|CommitAbility))
  (if _returnvalue
    (bind _returnvalue_2 (Game|SpawnActorfromClass "/Game/Fragmented/Characters/BP_FragmentedPlayerClone.BP_FragmentedPlayerClone_C" (Math|Transform|MakeTransform (Transformation|GetActorLocation (Ability|GetAvatarActorfromActorInfo)) "0, 0, 0" "1.000000,1.000000,1.000000") "AlwaysSpawn" "MultiplyWithRoot" 0 (Variables|Default|GetAs%20BP%20Fragmented%20Player)))
    (Default|AddClonetoPlayerArray (Variables|Default|GetAs%20BP%20Fragmented%20Player) _returnvalue_2)
    (Class|GameplayAbility|AddGameplayCuewithParams "(TagName=\"GameplayCue.AOEIndicator\")" (Ability|GameplayCue|MakeGameplayCueParameters :RawMagnitude (* (Variables|Default|GetAOERadius) 2.0) :Location (Variables|Default|GetComfirmedAOELocation)) true)
    (|PlayMontageandWaitProxy "None" "/Game/SwordAnimsetPro/Animations/In-Place/Buff_out_Anim_Montage.Buff_out_Anim_Montage" 1.0 "None" true 1.0 0.0 false
      (:then
        (Ability|Tasks|WaitGameplayEvent "(TagName=\"Event.Montage.Trigger\")" 0
          (:EventReceived
            (CallFunction|TeleporttoLocation)
            (Class|GameplayAbility|ExecuteGameplayCuewithParams "(TagName=\"GameplayCue.TeleportExplosion\")" (Ability|GameplayCue|MakeGameplayCueParameters :Location (Variables|Default|GetComfirmedAOELocation)))
            (CallFunction|AOEDamage)
            (GameplayCue|RemoveGameplayCue "(TagName=\"GameplayCue.AOEIndicator\")"))))
      (:OnCompleted
        (Ability|EndAbility :!label _label))
      (:OnInterrupted
        (goto _label)))
    (else
      (Ability|EndAbility))))

(event Custom|AOEDamage
  (bind _comfirmedaoelocation (Variables|Default|GetComfirmedAOELocation))
  ;[0.15 0.15 0.15 0.5] Phase 2
  (Ability|HasAuthority
    (:True
      (bind _outhits (Collision|MultiSphereTraceForObjects _comfirmedaoelocation _comfirmedaoelocation (Variables|Default|GetAOERadius) (Utilities|Array|MakeArray "ObjectTypeQuery3") false (Utilities|Array|MakeArray (Ability|GetAvatarActorfromActorInfo)) "None"))
      (Utilities|Array|Clear (Variables|Default|GetHitActors))
      (for _array_element _outhits
        (if (not (Utilities|Array|ContainsItem (Variables|Default|GetHitActors) (.HitActor (Collision|BreakHitResult _array_element))))
          (Utilities|Array|AddUnique (Variables|Default|GetHitActors) (.HitActor (Collision|BreakHitResult _array_element)))
          (Utilities|IsValid (Ability|GetAbilitySystemComponent (.HitActor (Collision|BreakHitResult _array_element)))
            (:Is%20Valid
              (bind _returnvalue (Ability|GameplayEffect|AssignTagSetbyCallerMagnitude (Ability|MakeOutgoingGameplayEffectSpec "/Game/Fragmented/Effects/GE_DamageInstant.GE_DamageInstant_C") "(TagName=\"Data.Damage\")" (Variables|Default|GetDamage%20Magnitude)))
              (GameplayEffects|ApplyGameplayEffectSpecToSelf (Ability|GetAbilitySystemComponent (.HitActor (Collision|BreakHitResult _array_element))) _returnvalue))))))))

(event Custom|TeleportToLocation
  (Transformation|Teleport (Variables|Default|GetAs%20BP%20Fragmented%20Player) (Variables|Default|GetComfirmedAOELocation) "0, 0, 0"))

(event Custom|StartTargeting
  (bind _aoeradius (Variables|Default|GetAOERadius))
  (bind _returnvalue (* _aoeradius 1.1))
  ;[0.15 0.15 0.15 0.5] Phase 1
  (bind _asbp_fragmented_player (Utilities|Casting|CastToBP_FragmentedPlayer (Ability|GetAvatarActorfromActorInfo)))
  (bind _output_get (Variables|Default|SetAs%20BP%20Fragmented%20Player _asbp_fragmented_player))
  (Utilities|IsValid (Variables|/Script/Engine.Character|GetCharacterMovement _output_get)
    (:Is%20Valid
      (bind _output_get_2 (Variables|Default|SetCharacter%20Movement (Variables|/Script/Engine.Character|GetCharacterMovement _output_get)))
      (Pawn|Components|CharacterMovement|SetMovementMode _output_get_2 "MOVE_None" 0)
      (if (Class|GameplayStatics|ObjectIsA (Pawn|GetController (.AsPawn (Utilities|Casting|CastToPawn (Ability|GetAvatarActorfromActorInfo)))) "/Script/Engine.PlayerController")
        (CallFunction|LoopTargetingAnimation)
        (Variables|Default|SetbIsWaitingTargetData true)
        (bind _data (|WaitTargetData :ConfirmationType "UserConfirmed" :Class "/Game/Fragmented/Abilities/TargetingActors/GA_TargetActorGroundTraceDecal.GA_TargetActorGroundTraceDecal_C" :Decal%20Size%20Y _returnvalue :Decal%20Size%20Z _returnvalue :Decal%20Material "/Game/Fragmented/Materials/M_CircleIndicator.M_CircleIndicator" :MaxRange 2e+03 :StartLocation (Class|GameplayAbility|MakeTargetLocationInfofromOwnerActor) :ReticleClass 0)
          (:ValidData
            (Variables|Default|SetbIsWaitingTargetData false)
            (Variables|Default|SetComfirmedAOELocation (.Location (Collision|BreakHitResult (Ability|TargetData|GetHitResultfromTargetData _data))))
            (CallFunction|ConfirmStrike)))
        (else
          (Ability|EndAbility))))))

(event Ability|EventActivateAbility
  (bind _attacktarget (Class|BPITargeting|GetAttackTarget(Message) (Ability|GetAvatarActorfromActorInfo)))
  (Utilities|IsValid _attacktarget
    (:Is%20Valid
      (bind _location (CallFunction|GetTargetGroundLocation _attacktarget))
      (Variables|Default|SetComfirmedAOELocation _location)
      (Variables|Default|SetCurrentLocation (Transformation|GetActorLocation (Ability|GetAvatarActorfromActorInfo)))
      (CallFunction|ConfirmStrike))
    (:Is%20Not%20Valid
      (CallFunction|StartTargeting))))

(event Ability|EventOnEndAbility
  (params (bWasCancelled :type Boolean)))

(fn GetTargetGroundLocation
  (params (Attack%20Target :type Actor%20Object%20Reference))
  (bind _returnvalue (Transformation|GetActorLocation Attack%20Target))
  (bind (_outhit _returnvalue_2) (Collision|LineTraceByChannel _returnvalue (- _returnvalue "0.000000,0.000000,999999.000000") "TraceTypeQuery1" false (Utilities|Array|MakeArray Attack%20Target) "None"))
  (return (.Location (Collision|BreakHitResult _outhit)) _returnvalue_2))