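; GA_Block is a Gameplay Ability that puts the avatar Character into a blocking stance.
; It commits, disables movement, then chains the block-in montage into a hold montage, restoring walking when the ability ends.
; Each hold applies a gameplay effect to the owner and waits for an Effects.Attack.Blocked event to play the hit reaction.
; Hold and hit montages loop back to the hold while IsStillBlocking is true; nothing here clears that flag.
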(event Ability|EventActivateAbility
  (bind _ascharacter (Utilities|Casting|CastToCharacter (Ability|GetAvatarActorfromActorInfo)))
  (bind _output_get (Variables|Default|SetAs%20Character _ascharacter))
  (bind _output_get_2 (Variables|Default|SetCharacter%20Movement (Variables|/Script/Engine.Character|GetCharacterMovement _output_get)))
  (Ability|CommitAbility)
  (Variables|Default|SetbIsStillBlocking true)
  (Pawn|Components|CharacterMovement|SetMovementMode _output_get_2 "MOVE_None" 0)
  (|PlayMontageandWaitProxy "None" "/Game/SwordAnimsetPro/Animations/In-Place/Block_In_Anim_Montage.Block_In_Anim_Montage" 1.0 "None" true 1.0 0.0 false
    (:OnCompleted
      _)
    (:OnBlendOut
      _))
  (|PlayMontageandWaitProxy "None" "/Game/SwordAnimsetPro/Animations/In-Place/Block_Hold_Anim_Montage.Block_Hold_Anim_Montage" 1.0 "None" true 1.0 0.0 false :!label _label
    (:then
      (Ability|ApplyGameplayEffectToOwner 0)
      (Ability|Tasks|WaitGameplayEvent "(TagName=\"Effects.Attack.Blocked\")" 0
        (:EventReceived
          (|PlayMontageandWaitProxy "None" "/Game/SwordAnimsetPro/Animations/In-Place/Block_Hit_Anim_Montage.Block_Hit_Anim_Montage" 1.0 "None" true 1.0 0.0 false
            (:OnCompleted
              _)
            (:OnBlendOut
              _)
            (:OnInterrupted
              _))
          (if (Variables|Default|GetbIsStillBlocking)
            (goto _label)))))
    (:OnCompleted
      (if (Variables|Default|GetbIsStillBlocking) :!label _label_2
        (goto _label)))
    (:OnBlendOut
      (goto _label_2))))

(event Ability|EventOnEndAbility
  (params (bWasCancelled :type Boolean))
  (Pawn|Components|CharacterMovement|SetMovementMode (Variables|Default|GetCharacter%20Movement) "MOVE_Walking" 0))