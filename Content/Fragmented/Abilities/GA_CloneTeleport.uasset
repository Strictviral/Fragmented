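; Gameplay ability that spawns a player clone playing an attack montage at the avatar's transform.
; After the montage starts, it waits for a clone event tag, spawns the clone and applies move-to-actor root motion targeting it.
; The target offset uses the last movement input, falling back to actor forward.
; A separate AbilityBaseSpawnClone function launches the clone along that direction, while SpawnClone defers to the parent.
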(event Ability|EventActivateAbility)

(event Ability|EventOnEndAbility
  (params (bWasCancelled :type Boolean)))

(event EventMontageStarted
  (Ability|Tasks|WaitGameplayEvent (Variables|Default|GetClone%20Ability%20Event%20Tag) 0
    (:EventReceived
      (bind _ascharacter (Utilities|Casting|CastToCharacter (Ability|GetAvatarActorfromActorInfo)))
      (Utilities|IsValid _ascharacter
        (:Is%20Valid
          (bind _returnvalue (Game|SpawnActorfromClass "/Game/Fragmented/Characters/BP_FragmentedPlayerClone.BP_FragmentedPlayerClone_C" (Transformation|GetActorTransform _ascharacter) "Undefined" "MultiplyWithRoot" 0 _ascharacter))
          (Animation|PlayAnimMontage _returnvalue "/Game/SwordAnimsetPro/Animations/Root-Motion/AnimationMontages/Combo2/Attack_Combo_02_02_Anim_Montage.Attack_Combo_02_02_Anim_Montage" 1.0 "None")
          (Ability|Tasks|ApplyRootMotionMoveToActorForce "None" _returnvalue (CallFunction|GetPlayerDirection) "AlignFromTargetToSource" 0.0 0 0 false "MOVE_Walking" false 0 0 "MaintainLastRootMotionVelocity"))))))

(event EventSpawnClone
  (|CallParentFunction))

(fn AbilityBaseSpawnClone
  (bind _ascharacter (Utilities|Casting|CastToCharacter (Ability|GetAvatarActorfromActorInfo)))
  (Utilities|IsValid _ascharacter
    (:Is%20Valid
      (bind _returnvalue (Game|SpawnActorfromClass "/Game/Fragmented/Characters/BP_FragmentedPlayerClone.BP_FragmentedPlayerClone_C" (Transformation|GetActorTransform _ascharacter) "Undefined" "MultiplyWithRoot" 0 _ascharacter))
      (Character|LaunchCharacter _returnvalue (* (CallFunction|GetPlayerDirection) 1e+03) true true)
      (Animation|PlayAnimMontage _returnvalue "/Game/SwordAnimsetPro/Animations/Root-Motion/AnimationMontages/Combo2/Attack_Combo_02_02_Anim_Montage.Attack_Combo_02_02_Anim_Montage" 1.0 "None"))))

(fn GetPlayerDirection
  (bind _aspawn (Utilities|Casting|CastToPawn (Ability|GetAvatarActorfromActorInfo))
    (:then
      (if (Math|Vector|VectorIsZero (Class|Pawn|GetLastMovementInputVector _aspawn))
        _
        (else
          (return (Class|Pawn|GetLastMovementInputVector _aspawn)))))
    (:CastFailed
      _))
  (return (Transformation|GetActorForwardVector (Ability|GetAvatarActorfromActorInfo))))