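; Gameplay ability that sacrifices the Fragmented player's active clones to grant a shield.
; On activation it destroys and counts every active clone, ending immediately if there are none.
; Otherwise it plays a montage, then on the trigger event commits, applies GE_GiveShield with the clone count as effect level and clears the clone array.
; Clones are destroyed before commit, and the count resets only on that event.
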(event Ability|EventActivateAbility
  (bind _asbp_fragmented_player (Utilities|Casting|CastToBP_FragmentedPlayer (Ability|GetOwningActorfromActorInfo)))
  (bind _output_get (Variables|Default|SetAs%20BP%20Fragmented%20Player _asbp_fragmented_player))
  (Utilities|IsValid _output_get
    (:Is%20Valid
      (for _array_element (Variables|/Game/Fragmented/Characters/BP_FragmentedPlayer.BP_FragmentedPlayer_C|GetActiveClones _output_get)
        (Math|Integer|IncrementInt (Variables|Default|GetCloneCount)
          (:%20%20
            (Actor|DestroyActor _array_element))))
      (if (> (Variables|Default|GetCloneCount) 0)
        (|PlayMontageandWaitProxy "None" "/Game/SwordAnimsetPro/Animations/Root-Motion/AnimationMontages/Combo1/Attack_Combo_01_03_Anim_Montage.Attack_Combo_01_03_Anim_Montage" 1.0 "None" true 1.0 0.0 false
          (:then
            (Ability|Tasks|WaitGameplayEvent "(TagName=\"Event.Montage.Trigger\")" 0
              (:EventReceived
                (Ability|CommitAbility)
                (Ability|ApplyGameplayEffectToOwner "/Game/Fragmented/Effects/GE_GiveShield.GE_GiveShield_C" (Variables|Default|GetCloneCount))
                (Variables|Default|SetCloneCount 0)
                (Default|ClearPlayerCloneArray (Variables|Default|GetAs%20BP%20Fragmented%20Player)))))
          (:OnCompleted
            (Ability|EndAbility :!label _label))
          (:OnInterrupted
            (goto _label))
          (:OnCancelled
            (goto _label)))
        (else
          (Ability|EndAbility))))
    (:Is%20Not%20Valid
      (Ability|EndAbility))))

(event Ability|EventOnEndAbility
  (params (bWasCancelled :type Boolean)))