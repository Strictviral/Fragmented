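; Gameplay ability that detonates the player's currently selected clone, damaging pawns around it.
; On activation it caches the clone's location, plays an attack montage and waits for the montage trigger event.
; The event runs an authority-only sphere trace, applying set-by-caller instant damage once per actor and firing the explosion cue only for hits with an ability system.
; It then destroys the clone and clears the player's reference.
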(event Custom|SelectAndExplodeClone
  (|PlayMontageandWaitProxy "None" "/Game/SwordAnimsetPro/Demo/AnimMontage/Air_Attack_06_Anim_Montage.Air_Attack_06_Anim_Montage" 1.0 "None" true 1.0 0.0 false
    (:OnCompleted
      _)
    (:OnBlendOut
      _)
    (:OnInterrupted
      _))
  (Ability|EndAbility))

(event Ability|EventActivateAbility
  (bind _asbp_fragmented_player (Utilities|Casting|CastToBP_FragmentedPlayer (Ability|GetAvatarActorfromActorInfo)))
  (bind _output_get (Variables|Default|SetAs%20BP%20Fragmented%20Player _asbp_fragmented_player))
  (Utilities|IsValid (Variables|/Game/Fragmented/Characters/BP_FragmentedPlayer.BP_FragmentedPlayer_C|GetCurrentActor _output_get)
    (:Is%20Valid
      (bind _output_get_2 (Variables|Default|SetCurrent%20Actor (Variables|/Game/Fragmented/Characters/BP_FragmentedPlayer.BP_FragmentedPlayer_C|GetCurrentActor _output_get)))
      (Variables|Default|SetCloneLocation (Transformation|GetActorLocation _output_get_2))
      (CallFunction|SelectandExplodeClone)
      (Ability|Tasks|WaitGameplayEvent "(TagName=\"Event.Montage.Trigger\")" 0
        (:EventReceived
          (CallFunction|SpawnExplosionatCloneLocation)
          (CallFunction|DeleteandCleanUpClone))))
    (:Is%20Not%20Valid
      (Ability|EndAbility))))

(event Ability|EventOnEndAbility
  (params (bWasCancelled :type Boolean)))

(fn SpawnExplosionatCloneLocation
  (bind _clonelocation (Variables|Default|GetCloneLocation))
  (Ability|HasAuthority
    (:True
      (bind _outhits (Collision|MultiSphereTraceForObjects _clonelocation _clonelocation (Variables|Default|GetAOERadius) (Utilities|Array|MakeArray "ObjectTypeQuery3") false (Utilities|Array|MakeArray (Ability|GetAvatarActorfromActorInfo)) "None"))
      (Utilities|Array|Clear (Variables|Default|GetHitActors))
      (for _array_element _outhits
        (if (not (Utilities|Array|ContainsItem (Variables|Default|GetHitActors) (.HitActor (Collision|BreakHitResult _array_element))))
          (Utilities|Array|AddUnique (Variables|Default|GetHitActors) (.HitActor (Collision|BreakHitResult _array_element)))
          (Utilities|IsValid (Ability|GetAbilitySystemComponent (.HitActor (Collision|BreakHitResult _array_element)))
            (:Is%20Valid
              (bind _returnvalue (Ability|GameplayEffect|AssignTagSetbyCallerMagnitude (Ability|MakeOutgoingGameplayEffectSpec "/Game/Fragmented/Effects/GE_DamageInstant.GE_DamageInstant_C") "(TagName=\"Data.Damage\")" (Variables|Default|GetDamage%20Magnitude)))
              (GameplayEffects|ApplyGameplayEffectSpecToSelf (Ability|GetAbilitySystemComponent (.HitActor (Collision|BreakHitResult _array_element))) _returnvalue)
              (Class|GameplayAbility|ExecuteGameplayCuewithParams "(TagName=\"GameplayCue.TeleportExplosion\")" (Ability|GameplayCue|MakeGameplayCueParameters :Location (Variables|Default|GetCloneLocation))))))))))

(fn DeleteandCleanUpClone
  (bind _current_actor (Variables|Default|GetCurrent%20Actor))
  (Utilities|IsValid _current_actor
    (:Is%20Valid
      (Class|BPIHighlight|SetHighlight(Message) _current_actor false)
      (Actor|DestroyActor (Variables|Default|GetCurrent%20Actor))
      (Variables|/Game/Fragmented/Characters/BP_FragmentedPlayer.BP_FragmentedPlayer_C|SetCurrentActor (Variables|Default|GetAs%20BP%20Fragmented%20Player) 0))))