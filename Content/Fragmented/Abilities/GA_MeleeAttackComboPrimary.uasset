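; Gameplay ability for the primary melee combo attack, which carries on only when combo input arrives inside a timed window.
; When the montage starts, it listens for ContinueCombo Start, End and Input gameplay events: Start opens the window and Input records whether it landed inside.
; End closes the window and ends the ability if no timely input was recorded.
; Hit-scan start is passed straight to the parent class.
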(event Ability|EventActivateAbility
  (|CallParentFunction) ; This node is disabled and will not be called.\nDrag off pins to build functionality.
)

(event Ability|EventOnEndAbility
  (params (bWasCancelled :type Boolean))
  (|CallParentFunction bWasCancelled) ; This node is disabled and will not be called.\nDrag off pins to build functionality.
)

(event EventMontageStarted
  (Ability|Tasks|WaitGameplayEvent "(TagName=\"Event.ContinueCombo.Start\")" 0
    (:then
      (Ability|Tasks|WaitGameplayEvent "(TagName=\"Event.ContinueCombo.End\")" 0
        (:then
          (Ability|Tasks|WaitGameplayEvent "(TagName=\"Event.ContinueCombo.Input\")" 0
            (:EventReceived
              (Variables|Default|SetbRecievedInputAtRightTime (Variables|Default|GetbIsWithinComboWindow)))))
        (:EventReceived
          (Variables|Default|SetbIsWithinComboWindow false)
          (if (not (Variables|Default|GetbRecievedInputAtRightTime))
            (Ability|EndAbility)))))
    (:EventReceived
      (Variables|Default|SetbIsWithinComboWindow true)
      (Variables|Default|SetbRecievedInputAtRightTime false))))

(event EventHandleHitScanStart
  (|CallParentFunction))