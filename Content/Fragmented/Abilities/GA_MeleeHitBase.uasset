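; Base melee attack gameplay ability that plays an attack montage on the player and drives the weapon's hit scanning.
; On the server, montage gameplay events open and close the scan window, handing the weapon a set-by-caller damage effect spec plus a second clone effect spec.
; The ability ends with the montage or when weapon or montage is invalid, closing any scan on end.
; Children hook MontageStarted for extra behavior.
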(event Custom|HandleHitScanStart
  ;[0.15 0.15 0.15 0.5] HitScanEvents
  (bind _playersweapon (Variables|PlayerInfo|GetPlayersWeapon)
    (:then
      (bind _returnvalue (Ability|GameplayEffect|AssignTagSetbyCallerMagnitude (Ability|MakeOutgoingGameplayEffectSpec (Variables|GameplayEffect|GetGameplay%20Effect%20Class)) "(TagName=\"Data.Damage\")" (Variables|GameplayEffect|GetDamageMagnitude)))
      (Default|HitScanStart _playersweapon _returnvalue (Ability|MakeOutgoingGameplayEffectSpec (Variables|Default|GetGameplay%20Effect%20Clone%20Class))))
    (:else)))

(event Custom|HandleHitScanEnd
  ;[0.15 0.15 0.15 0.5] HitScanEvents
  (bind _playersweapon (Variables|PlayerInfo|GetPlayersWeapon)
    (:then
      (Default|HitScanEnd _playersweapon))
    (:else)))

(event Custom|MontageStarted
  ;[0.15 0.15 0.15 0.5] Override In Child
)

(event Ability|EventActivateAbility
  ;[0.15 0.15 0.15 0.5] Initialize Default HitAbility
  (bind _asbp_fragmented_player (Utilities|Casting|CastToBP_FragmentedPlayer (Ability|GetAvatarActorfromActorInfo)))
  (bind _output_get (Variables|PlayerInfo|SetAs%20BP%20Fragmented%20Player _asbp_fragmented_player))
  (Utilities|IsValid (Variables|/Game/Fragmented/Characters/BP_FragmentedPlayer.BP_FragmentedPlayer_C|GetWeapon _output_get)
    (:Is%20Valid
      (Variables|PlayerInfo|SetPlayersWeapon (Variables|/Game/Fragmented/Characters/BP_FragmentedPlayer.BP_FragmentedPlayer_C|GetWeapon _output_get))
      (bind _attackmontage (Variables|Animation|GetAttackMontage)
        (:then
          (|PlayMontageandWaitProxy "None" _attackmontage 1.0 "None" true 1.0 0.0 false
            (:then
              (CallFunction|MontageStarted)
              (Ability|HasAuthority
                (:True
                  (Ability|Tasks|WaitGameplayEvent "(TagName=\"Event.HitScan.Start\")" 0
                    (:then
                      (Ability|Tasks|WaitGameplayEvent "(TagName=\"Event.HitScan.End\")" 0
                        (:EventReceived
                          (CallFunction|HandleHitScanEnd))))
                    (:EventReceived
                      (CallFunction|HandleHitScanStart))))))
            (:OnCompleted
              (Ability|EndAbility :!label _label))
            (:OnInterrupted
              (goto _label))
            (:OnCancelled
              (goto _label))))
        (:else
          (Ability|EndAbility :!label _label_2))))
    (:Is%20Not%20Valid
      (goto _label_2))))

(event Ability|EventOnEndAbility
  (params (bWasCancelled :type Boolean))
  ;[0.15 0.15 0.15 0.5] HitScanEvents
  (CallFunction|HandleHitScanEnd))