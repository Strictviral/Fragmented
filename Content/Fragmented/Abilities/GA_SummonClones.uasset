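; Gameplay ability that makes the avatar summon an army of clones through its BPC_CloneComponent.
; On activation it plays an attack combo montage and waits for the Event.Montage.Trigger gameplay event, then calls SummonArmyOfClone on the component.
; The ability ends when the montage completes or is interrupted, or immediately if the avatar has no clone component.
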(event Ability|EventActivateAbility
  (bind _output_get (Variables|Default|SetCloneComponent (Actor|GetComponentbyClass (Ability|GetAvatarActorfromActorInfo) "/Game/Fragmented/Components/BPC_CloneComponent.BPC_CloneComponent_C")))
  (Utilities|IsValid _output_get
    (:Is%20Valid
      (Development|PrintString "Hello")
      (|PlayMontageandWaitProxy "None" "/Game/SwordAnimsetPro/Animations/Root-Motion/AnimationMontages/Combo1/Attack_Combo_01_03_Anim_Montage.Attack_Combo_01_03_Anim_Montage" 1.0 "None" true 1.0 0.0 false
        (:then
          (Ability|Tasks|WaitGameplayEvent "(TagName=\"Event.Montage.Trigger\")" 0
            (:EventReceived
              (Default|SummonArmyOfClone (Variables|Default|GetCloneComponent)))))
        (:OnCompleted
          (Ability|EndAbility :!label _label))
        (:OnInterrupted
          (goto _label))))
    (:Is%20Not%20Valid
      (Development|PrintString "No component")
      (Ability|EndAbility))))

(event Ability|EventOnEndAbility
  (params (bWasCancelled :type Boolean)))