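; Gameplay ability that teleports the Fragmented player to the nearest active clone, ending immediately if none exist.
; Concurrent gameplay event listeners drive it: fade-out dissolves the player, fade-in reverses the dissolve, and the teleport event re-finds the closest clone and moves the player there.
; Ending the ability also reverses the dissolve.
; The SwapLocationsWithClone function, which would exchange both positions, is never called here.
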(event Ability|EventActivateAbility
  (|CallParentFunction)
  (if (== (Utilities|Array|Length (Variables|/Game/Fragmented/Characters/BP_FragmentedPlayer.BP_FragmentedPlayer_C|GetActiveClones (Variables|Default|GetAs%20BP%20Fragmented%20Player))) 0)
    (Ability|EndAbility)
    (else
      (CallFunction|FindClosetCloneandSet (CallFunction|ReturnArrayOfPlayerClones))
      (Ability|Tasks|WaitGameplayEvent "(TagName=\"GameplayAbility.Effect.Fade.IN\")" 0
        (:then
          (Ability|Tasks|WaitGameplayEvent "(TagName=\"GameplayAbility.Effect.Fade.OUT\")" 0
            (:then
              (Ability|Tasks|WaitGameplayEvent "(TagName=\"GameplayAbility.Movement.Teleport\")" 0
                (:EventReceived
                  (bind _closetclone (CallFunction|FindClosetCloneandSet (CallFunction|ReturnArrayOfPlayerClones)))
                  (Utilities|IsValid _closetclone
                    (:Is%20Valid
                      (Transformation|Teleport (Ability|GetAvatarActorfromActorInfo) (Transformation|GetActorLocation _closetclone) "0, 0, 0"))
                    (:Is%20Not%20Valid
                      (Ability|EndAbility))))))
            (:EventReceived
              (Default|Dissolve (Variables|Default|GetAs%20BP%20Fragmented%20Player)))))
        (:EventReceived
          (Default|ReverseDissolve (Variables|Default|GetAs%20BP%20Fragmented%20Player)))))))

(event EventOnEndAbility
  (params (bWasCancelled :type Boolean))
  (|CallParentFunction false)
  (Default|ReverseDissolve (Variables|Default|GetAs%20BP%20Fragmented%20Player)))

(fn SwapLocationswithClone
  (params (CloneActor :type Actor%20Object%20Reference) (PlayerActor :type Actor%20Object%20Reference))
  (Development|PrintString "Hello")
  (LocalVariables|SetCloneLocation (Transformation|GetActorLocation CloneActor))
  (LocalVariables|SetPlayerLocation (Transformation|GetActorLocation PlayerActor))
  (Transformation|Teleport PlayerActor (LocalVariables|GetCloneLocation) "0, 0, 0")
  (Transformation|Teleport CloneActor (LocalVariables|GetPlayerLocation) "0, 0, 0"))

(fn FindClosestClone
  (params (ActiveClones :type Array%20of%20BP%20Fragmented%20Player%20Clone%20Object%20References))
  (for _array_element ActiveClones
    (Utilities|IsValid _array_element
      (:Is%20Valid
        (if (< (Transformation|GetDistanceTo (Ability|GetAvatarActorfromActorInfo) _array_element) (Variables|Clone|GetMinDistance))
          (Variables|Clone|SetMinDistance (Transformation|GetDistanceTo (Ability|GetAvatarActorfromActorInfo) _array_element))
          (Variables|Clone|SetClosestClone _array_element)))
      (:Is%20Not%20Valid
        (Ability|EndAbility))))
  (Variables|Clone|SetMinDistance (Variables|Default|GetDefaultMinimumDistance))
  (return (Variables|Clone|GetClosestClone)))

(fn FindClosetCloneandSet
  (params (ActiveClones :type Array%20of%20BP%20Fragmented%20Player%20Clone%20Object%20References))
  (bind _closestclone (CallFunction|FindClosestClone ActiveClones))
  (bind _output_get (Variables|Clone|SetClosestClone _closestclone))
  (return _output_get))

(fn ReturnArrayOfPlayerClones
  (return (Variables|/Game/Fragmented/Characters/BP_FragmentedPlayer.BP_FragmentedPlayer_C|GetActiveClones (Variables|Default|GetAs%20BP%20Fragmented%20Player))))