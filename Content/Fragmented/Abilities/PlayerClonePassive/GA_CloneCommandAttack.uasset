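; Gameplay ability that commands a clone attack by spawning a clone at the player's currently targeted actor.
; On activation it reads the target from BP_FragmentedPlayer and finds the avatar's BPC_CloneComponent, ending immediately if any is invalid.
; It plays a combo attack montage, and the montage trigger gameplay event calls SpawnCloneAtTarget with zero radius.
; The ability ends after that spawn, or when the montage completes, blends out or is interrupted.
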(event Ability|EventActivateAbility
  (bind _returnvalue (Ability|GetAvatarActorfromActorInfo))
  (bind _returnvalue_2 (Actor|GetComponentbyClass _returnvalue "/Game/Fragmented/Components/BPC_CloneComponent.BPC_CloneComponent_C"))
  (bind _asbp_fragmented_player (Utilities|Casting|CastToBP_FragmentedPlayer _returnvalue)
    (:then
      (bind _output_get (Variables|Default|SetAs%20BP%20Fragmented%20Player _asbp_fragmented_player))
      (Utilities|IsValid (Variables|/Game/Fragmented/Characters/BP_FragmentedPlayer.BP_FragmentedPlayer_C|GetCurrentTargettedActor _output_get)
        (:Is%20Valid
          (Variables|Default|SetCurrent%20Targetted%20Actor (Variables|/Game/Fragmented/Characters/BP_FragmentedPlayer.BP_FragmentedPlayer_C|GetCurrentTargettedActor _output_get))
          (Utilities|IsValid _returnvalue_2
            (:Is%20Valid
              (Variables|Default|SetCloneComponent _returnvalue_2)
              (|PlayMontageandWaitProxy "None" "/Game/SwordAnimsetPro/Animations/Root-Motion/AnimationMontages/Combo2/Attack_Combo_02_02_Anim_Montage.Attack_Combo_02_02_Anim_Montage" 1.0 "None" true 1.0 0.0 false
                (:then
                  (Ability|Tasks|WaitGameplayEvent "(TagName=\"Event.Montage.Trigger\")" 0
                    (:EventReceived
                      (Default|SpawnCloneatTarget (Variables|Default|GetCloneComponent) (Variables|Default|GetCurrent%20Targetted%20Actor) 0.0)
                      (Ability|EndAbility))))
                (:OnCompleted
                  (Ability|EndAbility :!label _label))
                (:OnBlendOut
                  (goto _label))
                (:OnInterrupted
                  (goto _label))))
            (:Is%20Not%20Valid
              (Ability|EndAbility :!label _label_2))))
        (:Is%20Not%20Valid
          (goto _label_2))))
    (:CastFailed
      (goto _label_2))))

(event Ability|EventOnEndAbility
  (params (bWasCancelled :type Boolean)))