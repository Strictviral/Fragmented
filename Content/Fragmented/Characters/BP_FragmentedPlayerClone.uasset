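; Temporary clone of the Fragmented player that spawns with its own weapon and attacks.
; On BeginPlay it grants clone abilities, starts the teleport-attack listener and activates a random melee ability.
; A dissolve timeline on a dynamic material fades it in, then out when its lifespan timer destroys it and the weapon.
; It removes itself from the instigating player's clone array on EndPlay and supports custom-depth highlighting.
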(event Custom|LifeTimeUntilDeath
  ;[0.15 0.15 0.15 0.5] Death Timer
  (Utilities|Time|SetTimerbyEvent (delegate Custom|DestroyActor) (Variables|Default|GetCloneLifeSpan)))

(event Custom|DestroyActor
  ;[0.15 0.15 0.15 0.5] Death Timer
  (CallFunction|Dissolve)
  (Utilities|FlowControl|Delay 0.5)
  (Actor|DestroyActor)
  (Actor|DestroyActor (Variables|Default|GetWeapon)))

(event Custom|Dissolve
  ;[0.15 0.15 0.15 0.5] Dissolve Effect
  (bind _dissolvetrack (Timeline|Timeline PlayFromStart)
    (:Update
      (Rendering|Material|SetScalarParameterValue (Variables|Default|GetDissolveMaterial) "Fade" (Math|Float|Lerp 0.0 1.0 _dissolvetrack) :!class /Script/Engine.MaterialInstanceDynamic))))

(event Custom|ReverseDissolve
  ;[0.15 0.15 0.15 0.5] Dissolve Effect
  (bind _dissolvetrack (Timeline|Timeline ReverseFromEnd)
    (:Update
      (Rendering|Material|SetScalarParameterValue (Variables|Default|GetDissolveMaterial) "Fade" (Math|Float|Lerp 0.0 1.0 _dissolvetrack) :!class /Script/Engine.MaterialInstanceDynamic))))

(event Custom|RandomAttackAbilityAcivation
  (bind _abilitysystemcomponent (Variables|Default|GetAbilitySystemComponent))
  ;[0.15 0.15 0.15 0.5] Random Attack Activation
  (Utilities|IsValid _abilitysystemcomponent
    (:Is%20Valid
      (bind _outabilityhandles (GameplayAbilities|FindAllAbilitieswithTags _abilitysystemcomponent "(GameplayTags=((TagName=\"GameplayAbility.MeleeAttack\")))" true))
      (Class|AbilitySystemComponent|TryActivateAbility (Variables|Default|GetAbilitySystemComponent) (.OutItem (Utilities|Array|Random _outabilityhandles)) true))))

(event Custom|Initialize%20Weapon
  ;[0.15 0.15 0.15 0.5] Weapon Creation
  (bind _returnvalue (Game|SpawnActorfromClass "/Game/Divinity/Blueprints/BP_Weapon.BP_Weapon_C" (Transformation|GetSocketTransform (Variables|Character|GetMesh) "Weapon_RSocket" "RTS_World") "Undefined" "MultiplyWithRoot" 0 self))
  (bind _output_get (Variables|Default|SetWeapon _returnvalue))
  (Transformation|AttachComponentToComponent _output_get (Variables|Character|GetMesh) "Weapon_RSocket" "SnapToTarget" "SnapToTarget" "SnapToTarget" true))

(event EventBeginPlay
  (bind _mesh (Variables|Character|GetMesh))
  ;[0.15 0.15 0.15 0.5] Initialize
  (|CallParentFunction)
  (bind _asbp_fragmented_player (Utilities|Casting|CastToBP_FragmentedPlayer (Variables|Default|GetInstigator)))
  (Variables|Default|SetAs%20BP%20Fragmented%20Player _asbp_fragmented_player)
  (CallFunction|InitializeWeapon)
  (Class|FragmentedCharacterBase|InitializeAbilitySystemComponent)
  (Class|FragmentedCharacterBase|GrantAbilities (Variables|Default|GetCloneStartingAbilities))
  (Abilities|TryActivateAbilitybyClass (Variables|Default|GetAbilitySystemComponent) "/Game/Fragmented/Abilities/CloneAbilities/GA_CloneTeleport_Attack_Listener.GA_CloneTeleport_Attack_Listener_C" true)
  (CallFunction|RandomAttackAbilityAcivation)
  (CallFunction|LifeTimeUntilDeath)
  (bind _returnvalue (Rendering|Material|CreateDynamicMaterialInstance _mesh 0 (Rendering|Material|GetMaterial _mesh 0) "None" :!class /Script/Engine.PrimitiveComponent))
  (bind _output_get (Variables|Default|SetDissolveMaterial _returnvalue))
  (Rendering|Material|SetScalarParameterValue (Variables|Default|GetDissolveMaterial) "Fade" 1.0 :!class /Script/Engine.MaterialInstanceDynamic)
  (CallFunction|ReverseDissolve))

(event EventEndPlay
  (params (EndPlayReason :type EEndPlayReason%20Enum :default "Destroyed"))
  ;[0.15 0.15 0.15 0.5] Clear Self From Player Array On Death
  (Default|RemoveSpecificClonefromArray (Variables|Default|GetAs%20BP%20Fragmented%20Player) self))

(event EventSetHighlight
  (params (bIsHighlighted :type Boolean))
  ;[0.15 0.15 0.15 0.5] Highlight Interface
  (if bIsHighlighted
    (CallFunction|RenderCustomDepth)
    (else
      (CallFunction|DisableCustomDepth))))

(fn ConstructionScript)

(fn RenderCustomDepth
  (Rendering|SetRenderCustomDepth (Variables|Character|GetMesh) true))

(fn DisableCustomDepth
  (Rendering|SetRenderCustomDepth (Variables|Character|GetMesh) false))