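; Base enemy Blueprint that sets up a health bar widget and starting gameplay tags on BeginPlay, and removes the bar on death.
; It creates dynamic materials for up to two mesh slots, whose Fade parameter a timeline drives for dissolve, reversed for the spawn animation.
; Helper functions activate abilities by class through the Ability System Component and return player controller 0 as the attack target; SetHighlight is an empty stub.
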(event Custom|Dissolve
  (bind _dissolvematerial_2 (Variables|Default|GetDissolveMaterial_2))
  (bind _dissolvetrack (Timeline|DissolveTimeline PlayFromStart)
    (:Update
      (Rendering|Material|SetScalarParameterValue (Variables|Default|GetDissolveMaterial) "Fade" (Math|Float|Lerp 0.0 1.0 _dissolvetrack) :!class /Script/Engine.MaterialInstanceDynamic)
      (Utilities|IsValid _dissolvematerial_2
        (:Is%20Valid
          (Rendering|Material|SetScalarParameterValue _dissolvematerial_2 "Fade" (Math|Float|Lerp 0.0 1.0 _dissolvetrack) :!class /Script/Engine.MaterialInstanceDynamic))))))

(event Custom|ReverseDissolve
  (bind _dissolvematerial_2 (Variables|Default|GetDissolveMaterial_2))
  (bind _dissolvetrack (Timeline|DissolveTimeline Reverse)
    (:Update
      (Rendering|Material|SetScalarParameterValue (Variables|Default|GetDissolveMaterial) "Fade" (Math|Float|Lerp 0.0 1.0 _dissolvetrack) :!class /Script/Engine.MaterialInstanceDynamic)
      (Utilities|IsValid _dissolvematerial_2
        (:Is%20Valid
          (Rendering|Material|SetScalarParameterValue _dissolvematerial_2 "Fade" (Math|Float|Lerp 0.0 1.0 _dissolvetrack) :!class /Script/Engine.MaterialInstanceDynamic))))))

(event EventBeginPlay
  (bind _mesh (Variables|Character|GetMesh))
  (bind _mesh_2 (Variables|Character|GetMesh))
  (bind _returnvalue (Rendering|Material|GetMaterial _mesh_2 1))
  (|CallParentFunction)
  (bind _returnvalue_2 (UserInterface|CreateWidget "/Game/Fragmented/Widgets/Enemy/WBP_EnemyHealthBar.WBP_EnemyHealthBar_C" 0 self))
  (UserInterface|SetWidget (Variables|Default|GetHealth%20Bar%20Widget%20Component) _returnvalue_2)
  (Ability|GameplayEffect|AddLooseGameplayTags self (Variables|Default|GetStarting%20Gameplay%20Tags) true)
  (bind _returnvalue_3 (Rendering|Material|CreateDynamicMaterialInstance _mesh 0 (Rendering|Material|GetMaterial _mesh 0) "None" :!class /Script/Engine.PrimitiveComponent))
  (bind _output_get (Variables|Default|SetDissolveMaterial _returnvalue_3))
  (Rendering|Material|SetScalarParameterValue (Variables|Default|GetDissolveMaterial) "Fade" 0.0 :!class /Script/Engine.MaterialInstanceDynamic)
  (Utilities|IsValid _returnvalue
    (:Is%20Valid
      (bind _returnvalue_4 (Rendering|Material|CreateDynamicMaterialInstance _mesh_2 1 _returnvalue "None" :!class /Script/Engine.PrimitiveComponent))
      (bind _output_get_2 (Variables|Default|SetDissolveMaterial_2 _returnvalue_4))
      (Rendering|Material|SetScalarParameterValue (Variables|Default|GetDissolveMaterial_2) "Fade" 0.0 :!class /Script/Engine.MaterialInstanceDynamic))))

(event EventSetHighlight
  (params (bIsHighlighted :type Boolean)))

(event EventSpawnedAnimation
  (CallFunction|ReverseDissolve))

(event EventHandleDeath
  (|CallParentFunction)
  (bind _health_bar_widget_component (Variables|Default|GetHealth%20Bar%20Widget%20Component)
    (:then
      (Components|DestroyComponent _health_bar_widget_component))
    (:else)))

(fn ConstructionScript
  (|CallParentFunction))

(fn ActivateAbility
  (params (AbilitySystemComponent :type Ability%20System%20Component%20Object%20Reference) (Ability%20To%20Activate :type Gameplay%20Ability%20Class%20Reference))
  (bind _returnvalue (Abilities|TryActivateAbilitybyClass AbilitySystemComponent Ability%20To%20Activate true))
  (return _returnvalue))

(fn GetAttackTarget
  (return (Game|GetPlayerController 0)))