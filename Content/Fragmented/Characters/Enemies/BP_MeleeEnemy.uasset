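; BP_MeleeEnemy is a melee enemy that deals weapon hits to players through the Gameplay Ability System.
; Left and right HitScanStart events store an effect spec, clear the hit list and start a roughly 30 Hz looping timer, which HitScanEnd stops.
; Left and right scan events sphere-trace between weapon socket pairs for pawns, with debug drawing on.
; Each actor tagged Team.Player receives the stored effect once per swing.
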(event Custom|HitScan_L
  (CallFunction|DrawHitScanBoxandHit (Transformation|GetSocketLocation (Variables|Character|GetMesh) "WeaponHB_Start_L") (Transformation|GetSocketLocation (Variables|Character|GetMesh) "WeaponHB_End_L")))

(event Custom|HitScanStart_R
  (params (EffectSpecHandle :type Gameplay%20Effect%20Spec%20Handle%20Structure))
  (Variables|Default|SetEffect%20Spec%20Handle EffectSpecHandle)
  (Utilities|Array|Clear (Variables|Default|GetHitActors))
  (bind _returnvalue (Utilities|Time|SetTimerbyEvent (EventDispatchers|CreateEvent :!event Custom|HitScan_R) 0.033333 true))
  (Variables|Default|SetHitScanTimer _returnvalue))

(event Custom|HitScanEnd
  (Utilities|Time|ClearandInvalidateTimerbyHandle (Variables|Default|GetHitScanTimer)))

(event Custom|HitScan_R
  (CallFunction|DrawHitScanBoxandHit (Transformation|GetSocketLocation (Variables|Character|GetMesh) "WeaponHB_Start_R") (Transformation|GetSocketLocation (Variables|Character|GetMesh) "WeaponHB_End_R")))

(event Custom|HitScanStart_L
  (params (EffectSpecHandle :type Gameplay%20Effect%20Spec%20Handle%20Structure))
  (Variables|Default|SetEffect%20Spec%20Handle EffectSpecHandle)
  (Utilities|Array|Clear (Variables|Default|GetHitActors))
  (bind _returnvalue (Utilities|Time|SetTimerbyEvent (EventDispatchers|CreateEvent :!event Custom|HitScan_L) 0.033333 true))
  (Variables|Default|SetHitScanTimer _returnvalue))

(event EventBeginPlay
  (|CallParentFunction) ; This node is disabled and will not be called.\nDrag off pins to build functionality.
)

(event Collision|EventActorBeginOverlap
  (params (OtherActor :type Actor%20Object%20Reference)))

(event EventTick
  (params (DeltaSeconds :type Float%20%28single-precision%29)))

(fn ConstructionScript
  (|CallParentFunction))

(fn DrawHitScanBoxandHit
  (params (StartLocation :type Vector) (EndLocation :type Vector))
  (bind _outhits (Collision|MultiSphereTraceForObjects StartLocation EndLocation (Variables|Default|GetHitScanRadius) (Utilities|Array|MakeArray "ObjectTypeQuery3") false (Utilities|Array|MakeArray (Variables|Default|GetInstigator)) "ForOneFrame" true "(R=1.000000,G=0.000000,B=0.000000,A=1.000000)" "(R=0.000000,G=1.000000,B=0.000000,A=1.000000)" 0.1))
  (for _array_element _outhits
    (Utilities|IsValid (Ability|GetAbilitySystemComponent (.HitActor (Collision|BreakHitResult _array_element)))
      (:Is%20Valid
        (if (GameplayTags|HasMatchingGameplayTag (Ability|GetAbilitySystemComponent (.HitActor (Collision|BreakHitResult _array_element))) "(TagName=\"Team.Player\")")
          (if (not (Utilities|Array|ContainsItem (Variables|Default|GetHitActors) (.HitActor (Collision|BreakHitResult _array_element))))
            (Utilities|Array|AddUnique (Variables|Default|GetHitActors) (.HitActor (Collision|BreakHitResult _array_element)))
            (GameplayEffects|ApplyGameplayEffectSpecToSelf (Ability|GetAbilitySystemComponent (.HitActor (Collision|BreakHitResult _array_element))) (Variables|Default|GetEffect%20Spec%20Handle))))))))