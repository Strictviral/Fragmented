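; Actor component for the fragmented player that spawns clones and orders them to attack targets.
; Generic spawning places a clone at a forward distance with random sideways offset, at the player's height and facing them, then registers it with the player.
; Despite its name, SpawnCloneAtTarget spawns nothing: it sends a GAS TeleportAttack gameplay event with the target to up to three active clones, ignoring SpawnRadius.
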(event EventBeginPlay
  (bind _output_get (Variables|Default|SetOwningActor (Components|GetOwner)))
  (bind _asbp_fragmented_player (Utilities|Casting|CastToBP_FragmentedPlayer _output_get))
  (Variables|Default|SetAs%20BP%20Fragmented%20Player _asbp_fragmented_player))

(fn SpawnCloneGeneric
  (bind _output_get (LocalVariables|SetSpawn%20Location (CallFunction|GetRadomSpawnLocation)))
  (bind _returnvalue (Game|SpawnActorfromClass "/Game/Fragmented/Characters/BP_FragmentedPlayerClone.BP_FragmentedPlayerClone_C" (Math|Transform|MakeTransform (Math|Vector|MakeVector (.x _output_get) (.y _output_get) (.z (Transformation|GetActorLocation (Variables|Default|GetOwningActor)))) (Math|Rotator|MakeRotator (.roll (Math|Rotator|FindLookatRotation (Math|Vector|MakeVector (.x _output_get) (.y _output_get) (.z _output_get)) (Transformation|GetActorLocation (Variables|Default|GetOwningActor)))) 0.0 (.yaw (Math|Rotator|FindLookatRotation (Math|Vector|MakeVector (.x _output_get) (.y _output_get) (.z _output_get)) (Transformation|GetActorLocation (Variables|Default|GetOwningActor))))) "1.000000,1.000000,1.000000") "AlwaysSpawn" "MultiplyWithRoot" (Variables|Default|GetOwningActor) (Variables|Default|GetAs%20BP%20Fragmented%20Player)))
  (Default|AddClonetoPlayerArray (Variables|Default|GetAs%20BP%20Fragmented%20Player) _returnvalue))

(fn GetRadomSpawnLocation
  (bind _owningactor (Variables|Default|GetOwningActor))
  (bind _maxspawndistancesideoffset (Variables|Default|GetMaxSpawnDistanceSideOffset))
  (return (+ (+ (Transformation|GetActorLocation _owningactor) (* (Transformation|GetActorForwardVector _owningactor) (Variables|Default|GetSpawnDistanceFwd))) (* (Transformation|GetActorRightVector _owningactor) (Math|Random|RandomFloatinRange (* _maxspawndistancesideoffset -1.0) _maxspawndistancesideoffset)))))

(fn SpawnCloneatTarget
  (params (TargetActor :type Actor%20Object%20Reference) (Spawn%20Radius :type Float%20%28double-precision%29))
  (for _index (range 0 (Math|Integer|Min(Integer) (- (Utilities|Array|Length (Variables|/Game/Fragmented/Characters/BP_FragmentedPlayer.BP_FragmentedPlayer_C|GetActiveClones (Variables|Default|GetAs%20BP%20Fragmented%20Player))) 1) 2))
    (Ability|SendGameplayEventtoActor (Utilities|Array|Get(acopy) (Variables|/Game/Fragmented/Characters/BP_FragmentedPlayer.BP_FragmentedPlayer_C|GetActiveClones (Variables|Default|GetAs%20BP%20Fragmented%20Player)) _index) "(TagName=\"GameplayAbility.Clone.TeleportAttack\")" (Utilities|Struct|MakeGameplayEventData "(TagName=\"\")" (Components|GetOwner) TargetActor 0 0 "()" "(GameplayTags=)" "(GameplayTags=)" 0.0 "()"))))